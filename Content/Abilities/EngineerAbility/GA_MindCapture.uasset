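; Engineer gameplay ability that targets a mech character along the avatar's aim and applies gameplay effects tagged TriggerAbility.ResponseMe to it.
; An instant WaitTargetData task gets a location offset from the avatar along control rotation by DistanceToTrace.
; A valid mech hit commits the ability, applies the effects and ends it.
; Cancellation also ends it, but a hit on anything else leaves it active.
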(event `self.K2_ActivateAbility`
  (bind _asmech_game_character (cast `MechGameCharacter` (`self.GetAvatarActorFromActorInfo`))
    (:`then`
      (bind _gameplayabilitytargetinglocationinfo (make `GameplayAbilityTargetingLocationInfo` "LiteralTransform" (`KismetMathLibrary.Conv_VectorToTransform` (`Actor.K2_GetActorLocation` _asmech_game_character))))
      (bind (_asynctaskproxy _data) (`AbilityTask_WaitTargetData.WaitTargetData` "None" "Instant" (`self.TargetActor`) (make `GameplayAbilityTargetingLocationInfo` (break `GameplayAbilityTargetingLocationInfo` _gameplayabilitytargetinglocationinfo) (`KismetMathLibrary.MakeTransform` (+ (* (`KismetMathLibrary.Conv_RotatorToVector` (`Pawn.GetControlRotation` _asmech_game_character)) (`self.DistanceToTrace`)) (.location (`.LiteralTransform` (break `GameplayAbilityTargetingLocationInfo` _gameplayabilitytargetinglocationinfo)))) (.rotation (`.LiteralTransform` (break `GameplayAbilityTargetingLocationInfo` _gameplayabilitytargetinglocationinfo))) (.scale (`.LiteralTransform` (break `GameplayAbilityTargetingLocationInfo` _gameplayabilitytargetinglocationinfo)))) (`.SourceActor` (break `GameplayAbilityTargetingLocationInfo` _gameplayabilitytargetinglocationinfo)) (`.SourceComponent` (break `GameplayAbilityTargetingLocationInfo` _gameplayabilitytargetinglocationinfo)) (`.SourceAbility` (break `GameplayAbilityTargetingLocationInfo` _gameplayabilitytargetinglocationinfo)) (`.SourceSocketName` (break `GameplayAbilityTargetingLocationInfo` _gameplayabilitytargetinglocationinfo))) (struct) null)
        (:`ValidData`
          (bind (_returnvalue_bblockinghit _returnvalue_binitialoverlap _returnvalue_time _returnvalue_distance _returnvalue_location _returnvalue_impactpoint _returnvalue_normal _returnvalue_impactnormal _returnvalue_physmat _returnvalue_hitactor) (`GameplayStatics.BreakHitResult` (`AbilitySystemBlueprintLibrary.GetHitResultFromTargetData` _data)))
          (cast `MechGameCharacter` _returnvalue_hitactor)
          (`self.K2_CommitAbility`)
          (`self.ApplyGameplayEffectsToTargetWithTags` (struct :`TagName` "TriggerAbility.ResponseMe") _data)
          (`self.K2_EndAbility`))
        (:`Cancelled`
          (`self.K2_EndAbility`))))
    (:`CastFailed`
      (`self.K2_EndAbility`))))