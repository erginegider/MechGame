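; AI controller for a test drone that starts its behavior tree and feeds it targets through the Blackboard.
; A one-shot timer from BeginPlay delays RunAI, which runs TestDroneBehaviorTree_BP and seeds TargetLocation with a randomly jittered point ahead of the pawn, plus a NavExtend vector.
; UpdateTargetActor writes a supplied character to the TargetActor key and prints its name for debugging.
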(event `self.ReceiveBeginPlay`
  (bind _returnvalue (`KismetSystemLibrary.K2_SetTimerDelegate` (delegate `RunAI`) 2.0))
  (set `self.AIBeginTimerHandle` _returnvalue))

(event `RunAI`
  (bind _returnvalue (`self.K2_GetPawn`))
  (bind _blackboard (`self.Blackboard`))
  (bind (_returnvalue_x _returnvalue_y _returnvalue_z) (`KismetMathLibrary.BreakVector` (+ (`self.K2_GetActorLocation` _returnvalue) (* (`self.GetActorForwardVector` _returnvalue) 500.0))))
  (`self.RunBehaviorTree` "/Game/TestCharacter/TestDroneBehaviorTree_BP.TestDroneBehaviorTree_BP")
  (`BlackboardComponent.SetValueAsVector` _blackboard (`self.TargetLocation`) (`KismetMathLibrary.MakeVector` (+ _returnvalue_x (`KismetMathLibrary.RandomFloatInRange` -100.0 100.0)) (+ _returnvalue_y (`KismetMathLibrary.RandomFloatInRange` -100.0 100.0)) (+ _returnvalue_z (`KismetMathLibrary.RandomFloatInRange` -100.0 100.0))))
  (`BlackboardComponent.SetValueAsVector` _blackboard (`self.NavExtend`) (1000.0 1000.0 1000.0))
  (`KismetSystemLibrary.K2_ClearAndInvalidateTimerHandle` (`self.AIBeginTimerHandle`)))

(fn `UpdateTargetActor`
  (params (TargetCharacter :type "MechGameCharacter Object Reference"))
  (locals (TargetActor :type Name :default "TargetActor"))
  (`BlackboardComponent.SetValueAsObject` (`self.Blackboard`) (`local.TargetActor`) TargetCharacter)
  (`KismetSystemLibrary.PrintString` (`KismetSystemLibrary.GetDisplayName` TargetCharacter)))

(fn `UserConstructionScript`)