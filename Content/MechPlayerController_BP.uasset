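; Player controller that uses AI perception to show health and armor displays on mechs the player senses.
; A successful sense makes that MechGameCharacter's HealthArmorComponent visible, along with its children.
; A lost sense starts a short timer, not cancelled by re-sensing, that hides the display on the last updated actor and makes perception forget all targets.
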(event `self.ReceiveBeginPlay`)

(event `self.ReceiveTick`
  (params (DeltaSeconds :type "Float (single-precision)")))

(event `self.PerceptionComponent.OnTargetPerceptionUpdated`
  (params (Actor :type "Actor Object Reference") (Stimulus :type "AIStimulus Structure"))
  (if Stimulus_bSuccessfullySensed
    (`self.UpdateUI` Actor true)
    (else
      (`KismetSystemLibrary.K2_SetTimerDelegate` (delegate `CloseUI`) 3.0))))

(event `CloseUI`
  (`self.UpdateUI` (stale `self.PerceptionComponent.OnTargetPerceptionUpdated` Actor))
  (`AIPerceptionComponent.ForgetAll` (`self.PerceptionComponent`)))

(fn `UpdateUI`
  (params (Actor :type "Actor Object Reference") (NewVisibility :type Boolean))
  (locals (NetRole :type "ENetRole Enum" :default "ROLE_SimulatedProxy"))
  (bind _asmech_game_character (cast `MechGameCharacter` Actor))
  (if true
    (`SceneComponent.SetVisibility` (`MechGameCharacter.HealthArmorComponent` _asmech_game_character) NewVisibility true)))

(fn `UserConstructionScript`)